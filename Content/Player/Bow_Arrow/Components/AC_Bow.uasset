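; Actor component that gives a Character a bow: equips it, handles aiming, drawing and firing arrows.
; Aiming switches rotation to controller-facing and spawns a socketed arrow, while a looping timer accumulates draw time and broadcasts it through dispatchers.
; Firing launches the arrow toward a camera line-trace target, with strength from normalized draw time.
; A draw requested while unavailable is buffered and resumes after the fire montage if still aiming.
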(event `self.ReceiveBeginPlay`
  ;[1 0.4902 0.9351] Gets The Character Ref
  (bind _ascharacter (cast `Character` (`self.GetOwner`)))
  (set `self.Character Ref` _ascharacter)
  (`self.EquipBow`)
  ;[0.05404 0.05404 0.05404] Initial Values always set from character start
  (set `self.Initial Rotation Rate` (`CharacterMovementComponent.RotationRate` (`Character.CharacterMovement` (`self.Character Ref`)))))

(event `Aim Starts`
  (bind _charactermovement (`Character.CharacterMovement` (`self.Character Ref`)))
  ;[1 0.4303 0.1956] Aim Bow and Player Rotation
  (set `self.isAiming` true)
  (set `CharacterMovementComponent.bUseControllerDesiredRotation` true _charactermovement)
  (set `CharacterMovementComponent.bOrientRotationToMovement` false _charactermovement)
  (set `CharacterMovementComponent.RotationRate` (`self.Aim Rotation Rate`) _charactermovement)
  (set `/Game/Player/Bow_Arrow/Bow/Bow_Blueprint/BP_Bow.BowState` "NewEnumerator1" (`self.Bow Ref`))
  (`self.SpawnArrow`)
  (`self.OnAimBegin`))

(event `Aim Ends`
  (bind _charactermovement (`Character.CharacterMovement` (`self.Character Ref`)))
  ;[1 0.4303 0.1956] Aim Bow and Player Rotation
  (set `self.isAiming` false)
  (`self.DrawBowEnd`) ; When we end the aim, naturally the draw also has to end
  (set `CharacterMovementComponent.bUseControllerDesiredRotation` false _charactermovement)
  (set `CharacterMovementComponent.bOrientRotationToMovement` true _charactermovement)
  (set `CharacterMovementComponent.RotationRate` (`self.Initial Rotation Rate`) _charactermovement)
  (set `/Game/Player/Bow_Arrow/Bow/Bow_Blueprint/BP_Bow.BowState` "NewEnumerator0" (`self.Bow Ref`))
  (`self.DestroyArrow`)
  (`self.OnAimEnds`))

(event `DrawBowBegin`
  ;[1 0.5651 0.9622] Draw Bow
  (`self.CanDrawBow?`
    (:`Yes`
      (set `self.IsWaitingToDrawBow` false) ; This Just Clears up the Input Buffering
      (set `self.IsDrawingBow?` true)
      (bind _returnvalue (`KismetSystemLibrary.K2_SetTimerDelegate` (delegate `IncrementDrawTIme`) (`self.DrawIncrementTime`) true))
      (set `self.DrawBowTimer` _returnvalue) ; In order to Clear the timer, we set it as a variable
      (`/Game/Player/Bow_Arrow/Bow/Bow_Blueprint/BP_Bow.DraawBegin` (`self.Bow Ref`)))
    (:`No`
      (set `self.IsWaitingToDrawBow` true) ; This Just Clears up the Input Buffering
    )))

(event `IncrementDrawTIme`
  ;[1 0.5651 0.9622] Draw Bow
  (bind _output_get (set `self.DrawTime` (+ (`self.DrawTime`) (`self.DrawIncrementTime`))))
  (`self.OnDrawOngoing` (`/Game/Player/Bow_Arrow/Bow/Bow_Blueprint/BP_Bow.MaxDrawTime` (`self.Bow Ref`)) _output_get) ; Everyrime this timer event is executed, we call this dispatcher to listen and call widget
)

(event `DrawBowEnd`
  ;[1 0.5651 0.9622] Draw Bow
  (set `self.IsDrawingBow?` false)
  (set `self.IsWaitingToDrawBow` false) ; This Just Clears up the Input Buffering
  (set `self.DrawTime` 0.0) ; Sets time back to zero
  (`KismetSystemLibrary.K2_ClearAndInvalidateTimerHandle` (`self.DrawBowTimer`)) ; Stops the timer from running
  (`/Game/Player/Bow_Arrow/Bow/Bow_Blueprint/BP_Bow.DraawEnd` (`self.Bow Ref`))
  (`self.OnDrawEnd`))

(event `FiringArrowBegin`
  ;[0.4629 1 0.329] Fire Arrow
  (if (`self.IsDrawingBow?`)
    (set `self.Isfiringarrow?` true)
    (`self.FireAimedArrow`)
    (`self.DrawBowEnd`)
    (`|PlayMontage` (`Character.Mesh` (`self.Character Ref`)) (`self.Fire Montage`)
      (:`OnCompleted`
        _)
      (:`OnInterrupted`
        _))
    (`self.FiringArrowEnd`)))

(event `FiringArrowEnd`
  ;[0.4629 1 0.329] Fire Arrow
  (set `self.Isfiringarrow?` false)
  (if (`self.isAiming`)
    (`self.Aim Starts`)
    (if (`self.IsWaitingToDrawBow`)
      (`self.DrawBowBegin`))))

(fn `ArrowTrajectoryCalculation`
  (returns (Direction :type "Vector Structure"))
  (bind _returnvalue (`Actor.GetComponentByClass` (`self.Character Ref`) "/Script/Engine.CameraComponent"))
  (bind _returnvalue_2 (`SceneComponent.K2_GetComponentLocation` _returnvalue))
  (bind (_outhit _returnvalue_3) (`KismetSystemLibrary.LineTraceSingle` _returnvalue_2 (+ _returnvalue_2 (* (`SceneComponent.GetForwardVector` _returnvalue) 10000.0)) "TraceTypeQuery1"))
  (bind _arrow_ref (`self.Arrow Ref`)
    (:`then`
      (bind (_bblockinghit _binitialoverlap _time _distance _location _impactpoint _normal _impactnormal _physmat _hitactor _hitcomponent _hitbonename _bonename _hititem _elementindex _faceindex _tracestart _traceend) (`GameplayStatics.BreakHitResult` _outhit))
      (return (`KismetMathLibrary.GetDirectionUnitVector` (`Actor.K2_GetActorLocation` _arrow_ref) (`KismetMathLibrary.SelectVector` _location _traceend _returnvalue_3))))
    (:`else`)))

(fn `DestroyArrow`
  (bind _arrow_ref (`self.Arrow Ref`)
    (:`then`
      (`Actor.K2_DestroyActor` _arrow_ref))
    (:`else`)))

(fn `EquipBow`
  (bind _returnvalue (`|SpawnActorFromClass` (`self.Bow Class`) (`KismetMathLibrary.MakeTransform` (0.0 0.0 0.0)) "AdjustIfPossibleButAlwaysSpawn" "MultiplyWithRoot" null null))
  (bind _output_get (set `self.Bow Ref` _returnvalue))
  (`Actor.K2_AttachToComponent` _output_get (`Character.Mesh` (`self.Character Ref`)) (`self.Bow Socket Name`) "SnapToTarget" "SnapToTarget" "SnapToTarget" true))

(fn `FireAimedArrow`
  (bind _arrow_ref (`self.Arrow Ref`)
    (:`then`
      (`Actor.K2_DetachFromActor` _arrow_ref "KeepWorld" "KeepWorld" "KeepWorld")
      (bind _direction (`self.ArrowTrajectoryCalculation`))
      (`/Game/Player/Bow_Arrow/Arrow/Actor/BP_Arrow.FireArrow` _arrow_ref _direction (`KismetMathLibrary.FClamp` (`KismetMathLibrary.NormalizeToRange` (`self.DrawTime`) 0.0 (`/Game/Player/Bow_Arrow/Bow/Bow_Blueprint/BP_Bow.MaxDrawTime` (`self.Bow Ref`))))) ; Fires teh arrow based on direction and Strength(draw time)
      (set `self.Arrow Ref` null) ; Resets the arrow ref from fired
    )
    (:`else`)))

(fn `SpawnArrow`
  (bind _returnvalue (`|SpawnActorFromClass` (`self.Arrow Class`) (`KismetMathLibrary.MakeTransform` (0.0 0.0 0.0)) "Undefined" "MultiplyWithRoot" null (`self.Character Ref`)))
  (bind _output_get (set `self.Arrow Ref` _returnvalue))
  (`Actor.K2_AttachToComponent` _output_get (`Character.Mesh` (`self.Character Ref`)) (`self.Arrow Socket Name`) "SnapToTarget" "SnapToTarget" "SnapToTarget" true))