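; Arrow projectile actor for the player's bow, with collision off until it is fired.
; FireArrow adds a projectile movement component at runtime, scales speed up and gravity down with draw strength, attaches a Niagara trail and sets a limited lifespan.
; On overlap with anything but its instigator, it stops, sticks to the hit component, plays impact effects and pushes physics-simulating bodies with its stored launch velocity.
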(event `self.ReceiveBeginPlay`
  (`PrimitiveComponent.SetCollisionEnabled` (`self.CollisionArrow`) "NoCollision") ; This Prevents ANy Collision By Default
)

(event `FireArrow`
  (params (Direction :type "Vector Structure") (Strength :type "Float (double-precision)"))
  (bind _returnvalue (`AddComponent|NODE_AddProjectileMovementComponent-0`))
  (bind _output_get (set `self.ProjectileMovementComponent` _returnvalue))
  (bind _output_get_2 (set `MovementComponent.Velocity` (* Direction (`KismetMathLibrary.Lerp` (`self.MinSpeed`) (`self.MaxSpeed`) Strength)) _output_get))
  (set `self.Velocity` _output_get_2) ; Ref of Velocity Vsriable
  (set `ProjectileMovementComponent.ProjectileGravityScale` (`KismetMathLibrary.Lerp` (`self.MaxGravity`) (`self.MinGravity`) Strength) _output_get)
  (`GameplayStatics.PlaySoundAtLocation` (`self.WhooshArrowSound`) (`self.K2_GetActorLocation`) (struct) 1.0 1.0 0.0 null null null null)
  (bind _returnvalue_2 (`NiagaraFunctionLibrary.SpawnSystemAttached` (`self.TrailEffect`) (`self.TrailEffectLocation`) "None" (0.0 0.0 0.0) (struct) "KeepRelativeOffset")) ; Spawn System - Niagara System and this spawn at the attached scene
  (set `self.TrailEffectRef` _returnvalue_2)
  (`PrimitiveComponent.SetCollisionEnabled` (`self.CollisionArrow`) "QueryAndPhysics")
  (`self.SetLifeSpan` 7.0))

(event `self.CollisionArrow.OnComponentBeginOverlap`
  (params (OverlappedComponent :type "PrimitiveComponent Object Reference") (OtherActor :type "Actor Object Reference") (OtherComp :type "PrimitiveComponent Object Reference") (OtherBodyIndex :type Integer) (bFromSweep :type Boolean) (SweepResult :type "HitResult Structure (by ref)"))
  (bind (_bblockinghit _binitialoverlap _time _distance _location _impactpoint _normal _impactnormal _physmat _hitactor _hitcomponent) (`GameplayStatics.BreakHitResult` SweepResult))
  (if (!= OtherActor (`self.GetInstigator`))
    (bind _projectilemovementcomponent (`self.ProjectileMovementComponent`)
      (:`then`
        (`ActorComponent.K2_DestroyComponent` _projectilemovementcomponent) ; In order to Collide with Something, the projectile movement component should first be destroyed.
      )
      (:`else`
        _))
    (`PrimitiveComponent.SetCollisionEnabled` (`self.CollisionArrow`) "NoCollision") ; Once Collided, then stop further collisions
    (`self.K2_AttachToComponent` _hitcomponent "None" "KeepWorld" "KeepWorld" "KeepWorld") ; This Attaches the Arrow to Whatever it collided with, make sure to keep that location as ref
    (`GameplayStatics.SpawnEmitterAtLocation` (`self.Impact Effect`) _location) ; This is Typically for Cascade Legacy Particle Effects
    (`GameplayStatics.PlaySoundAtLocation` (`self.ImpactSound`) (`self.K2_GetActorLocation`) (struct) 1.0 1.0 0.0 null null null null)
    (if (`SceneComponent.IsSimulatingPhysics` _hitcomponent "None")
      (`PrimitiveComponent.AddImpulse` _hitcomponent (`self.Velocity`) "None" true))
    (`KismetSystemLibrary.Delay` 1.0)
    (bind _traileffectref (`self.TrailEffectRef`)
      (:`then`
        (`ActorComponent.K2_DestroyComponent` _traileffectref))
      (:`else`))))

(fn `UserConstructionScript`)